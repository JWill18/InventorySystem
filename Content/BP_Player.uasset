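; First-person player Blueprint with item pickup and a toggleable inventory menu.
; A short camera line trace each tick highlights the ItemActor in view, and E adds it to an Inventory object created at BeginPlay, then destroys the actor.
; Tab shows or hides a lazily created, repopulated W_InventoryList with the mouse cursor.
; An open-menu flag blocks look, movement and pickup, as the UI-only input mode node is disconnected.
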(event EventBeginPlay
  ;[1 1 1] Instantiate Inventory
  (bind _returnvalue (Game|ConstructObjectfromClass "/Script/InventorySystem.Inventory" self))
  (Variables|Default|SetInventory _returnvalue))

(event Collision|EventActorBeginOverlap
  (params (OtherActor :type Actor%20Object%20Reference)))

(event EventTick
  (params (DeltaSeconds :type Float%20%28single-precision%29))
  (bind _camera (Variables|Default|GetCamera))
  (bind _returnvalue (Transformation|GetWorldLocation _camera))
  ;[1 1 1] Check for collision with other objects based on where the camera is looking
  (bind _outhit (Collision|LineTraceByChannel _returnvalue (+ _returnvalue (* (Math|Vector|GetForwardVector (Variables|Default|GetCamera)) 1.5e+02)) "TraceTypeQuery1" false 0 "None"))
  ;[1 1 1] Highlight itemActor and unhighlight old itemActor
  (bind _asitem_actor (Utilities|Casting|CastToItemActor (.hitactor _outhit))
    (:then
      (if (== (Variables|Default|GetItemTarget) 0)
        _
        (else
          (Class|ItemActor|HighlightItem (Variables|Default|GetItemTarget) false)))
      (bind _output_get (Variables|Default|SetItemTarget _asitem_actor))
      (Class|ItemActor|HighlightItem _output_get true))
    (:CastFailed
      (if (!= (Variables|Default|GetItemTarget) 0)
        (Class|ItemActor|HighlightItem (Variables|Default|GetItemTarget) false)
        (Variables|Default|SetItemTarget 0)))))

(event Input|AxisEvents|InputAxisMoveForward
  (params (AxisValue :type Float%20%28single-precision%29))
  ;[1 1 1] Player Movement
  (if (not (Variables|Default|GetIsInventoryOpen))
    (Pawn|Input|AddMovementInput (Math|Vector|GetForwardVector (Variables|Default|GetCamera)) AxisValue false)))

(event Input|AxisEvents|InputAxisMoveSideways
  (params (AxisValue :type Float%20%28single-precision%29))
  ;[1 1 1] Player Movement
  (if (not (Variables|Default|GetIsInventoryOpen))
    (Pawn|Input|AddMovementInput (Math|Vector|GetRightVector (Variables|Default|GetCamera)) AxisValue false)))

(event Input|MouseEvents|MouseX
  (params (AxisValue :type Float%20%28single-precision%29))
  ;[1 1 1] Camera Movement
  (if (not (Variables|Default|GetIsInventoryOpen))
    (Pawn|Input|AddControllerYawInput AxisValue)))

(event Input|MouseEvents|MouseY
  (params (AxisValue :type Float%20%28single-precision%29))
  ;[1 1 1] Camera Movement
  (if (not (Variables|Default|GetIsInventoryOpen))
    (Pawn|Input|AddControllerPitchInput (* AxisValue -1.0))))

(event Input|KeyboardEvents|E
  (params (Key :type Key%20Structure))
  ;[1 1 1] Pickup item and place it into the the inventory
  (:Pressed
    (if (not (Variables|Default|GetIsInventoryOpen))
      (if (!= (Variables|Default|GetItemTarget) 0)
        (Class|Inventory|AddItem (Variables|Default|GetInventory) (Variables|Default|GetItemTarget))
        (Actor|DestroyActor (Variables|Default|GetItemTarget))
        (Variables|Default|SetItemTarget 0)))))

(event Input|KeyboardEvents|Tab
  (params (Key :type Key%20Structure))
  (bind _returnvalue (Game|GetPlayerController 0))
  ;[1 1 1] Opening and closing the inventory menu
  (:Pressed
    (if (Variables|Default|GetIsInventoryOpen)
      (Widget|RemovefromParent (Variables|Default|GetInventoryMenu))
      (Variables|Default|SetIsInventoryOpen false)
      (Variables|/Script/Engine.PlayerController|SetbShowMouseCursor _returnvalue false)
      (Input|SetInputModeGameOnly _returnvalue)
      (else
        (if (== (Variables|Default|GetInventoryMenu) 0)
          (bind _returnvalue_2 (UserInterface|CreateWidget "/Game/Inventory/Widgets/W_InventoryList.W_InventoryList_C"))
          (Variables|Default|SetInventoryMenu _returnvalue_2))
        (UserInterface|Viewport|AddtoViewport (Variables|Default|GetInventoryMenu) 0)
        (Default|PopulateList (Variables|Default|GetInventoryMenu))
        (Variables|/Script/Engine.PlayerController|SetbShowMouseCursor (Game|GetPlayerController 0) true)
        (Variables|Default|SetIsInventoryOpen true)))))

(fn ConstructionScript)